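; BP_Chrono is a countdown timer that starts automatically on BeginPlay and displays the remaining time on screen.
; BeginPlay sets the current time from BaseTime, then creates a BP_ChronoUi widget and adds it to the viewport.
; While running, Tick subtracts delta seconds, pushes the value to the widget, and stops the timer once it reaches zero or below.
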(event Custom|Start%20Chrono
  (params (BaseTime :type Float%20%28double-precision%29))
  (Variables|Default|SetCurrentTime BaseTime)
  (Variables|Default|SetIsTimerStarted true))

(event Custom|Stop%20Chrono
  (Variables|Default|SetIsTimerStarted false))

(event EventTick
  (params (DeltaSeconds :type Float%20%28single-precision%29))
  (if (Variables|Default|GetIsTimerStarted)
    (bind _output_get (Variables|Default|SetCurrentTime (- (Variables|Default|GetCurrentTime) DeltaSeconds)))
    (Default|SetText (Variables|Default|GetUI) _output_get)
    (if (<= (Variables|Default|GetCurrentTime) 0.0)
      (CallFunction|StopChrono))))

(event EventBeginPlay
  (CallFunction|StartChrono (Variables|Default|GetBaseTime))
  (bind _returnvalue (Game|ConstructObjectfromClass "/Game/TalesRun/Devs/BP_ChronoUi.BP_ChronoUi_C"))
  (bind _output_get (Variables|Default|SetUI _returnvalue))
  (UserInterface|Viewport|AddtoViewport _output_get 0))