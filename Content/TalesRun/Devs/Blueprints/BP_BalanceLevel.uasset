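; BP_BalanceLevel is a per-level tuning actor that pushes gameplay balance values onto the player character and trampolines at start.
; After a short delay on BeginPlay, it finds the BP_Character_Devi instance and sets its walk speed, jump velocity, invincibility time and maximum slide duration.
; It then loops over every BP_Chamalow_Trampoline in the level, setting each vertical launch force from its own variable.
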(event EventBeginPlay
  (Utilities|FlowControl|Delay 0.2)
  (bind _returnvalue (Actor|GetActorOfClass "/Game/TalesRun/Devs/Blueprints/BP_Character_Devi.BP_Character_Devi_C"))
  (Variables|/Script/Engine.CharacterMovementComponent|SetMaxWalkSpeed (Variables|/Script/Engine.Character|GetCharacterMovement _returnvalue) (Variables|Default|GetCharacterSpeed))
  (Variables|/Script/Engine.CharacterMovementComponent|SetJumpZVelocity (Variables|/Script/Engine.Character|GetCharacterMovement _returnvalue) (Variables|Default|GetCharacterJump))
  (Variables|/Game/TalesRun/Devs/Blueprints/BP_Character_Devi.BP_Character_Devi_C|SetInvincibilityTime _returnvalue (Variables|Default|GetCharacterInvincibilityTime))
  (Variables|/Game/TalesRun/Devs/Blueprints/BP_Character_Devi.BP_Character_Devi_C|SetMaxSecondsSlide _returnvalue (Variables|Default|GetSlideMaxSeconds))
  (bind _outactors (Actor|GetAllActorsOfClass "/Game/TalesRun/Devs/Blueprints/Traps/BP_Chamalow_Trampoline.BP_Chamalow_Trampoline_C"))
  (bind _array_element (Utilities|Array|ForEachLoopwithBreak _outactors)
    (:LoopBody
      (Variables|/Game/TalesRun/Devs/Blueprints/Traps/BP_Chamalow_Trampoline.BP_Chamalow_Trampoline_C|SetLaunchForce _array_element (Math|Vector|MakeVector 0.0 0.0 (Variables|Default|GetChamallowJumpForce))))))

(event Collision|EventActorBeginOverlap
  (params (OtherActor :type Actor%20Object%20Reference)))

(event EventTick
  (params (DeltaSeconds :type Float%20%28single-precision%29)))

(fn ConstructionScript)