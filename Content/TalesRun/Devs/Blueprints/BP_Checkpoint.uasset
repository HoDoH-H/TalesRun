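; BP_Checkpoint is a trigger actor that teleports the main character to its TargetDestination component behind a circular screen fade.
; On overlap it removes the character's in-game UI, adds WBP_FadeCircular and drives its dynamic material's Fade parameter with the FadeAnim timeline.
; When that finishes it moves the character, then ReverseAnim waits briefly, runs a second fade timeline, removes the widget and calls the character's ClosePauseMenu.
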(event OnComponentBeginOverlap(Trigger)
  (params (OverlappedComponent :type Primitive%20Component%20Object%20Reference) (OtherActor :type Actor%20Object%20Reference) (OtherComp :type Primitive%20Component%20Object%20Reference) (OtherBodyIndex :type Integer) (bFromSweep :type Boolean) (SweepResult :type Hit%20Result%20Structure%20%28by%20ref%29))
  (bind (_castsuccess _iscapsulecomponent _characterref) (CallFunction|CasttoMainCharacter OtherActor OtherComp))
  (if _castsuccess
    (bind _output_get (Variables|Default|SetCharacter%20Ref _characterref))
    (Widget|RemovefromParent (Variables|/Game/TalesRun/Devs/Blueprints/BP_Character_Devi.BP_Character_Devi_C|GetInGameUI _output_get))
    (bind _returnvalue (UserInterface|CreateWidget "/Game/TalesRun/Devs/Blueprints/TransitionCheckpoint/WBP_FadeCircular.WBP_FadeCircular_C" (Game|GetPlayerController 0)))
    (bind _output_get_2 (Variables|Default|SetFadeWidget _returnvalue))
    (UserInterface|Viewport|AddtoViewport _output_get_2 0)
    (bind _returnvalue_2 (Appearance|GetDynamicMaterial (Variables|/Game/TalesRun/Devs/Blueprints/TransitionCheckpoint/WBP_FadeCircular.WBP_FadeCircular_C|GetFadeImage (Variables|Default|GetFadeWidget)) :!class /Script/UMG.Image))
    (Variables|Default|SetFadeMaterial _returnvalue_2)
    (bind _fadevalue (Timeline|FadeAnim PlayFromStart)
      (:Update
        (Rendering|Material|SetScalarParameterValue (Variables|Default|GetFadeMaterial) "Fade" _fadevalue :!class /Script/Engine.MaterialInstanceDynamic))
      (:Finished
        (Transformation|SetActorLocation (Variables|Default|GetCharacter%20Ref) (Transformation|GetWorldLocation (Variables|Default|GetTargetDestination)) false true)
        (CallFunction|ReverseAnim)))))

(event Custom|ReverseAnim
  (Utilities|FlowControl|Delay 0.2)
  (bind _fadevalue (Timeline|Timeline PlayFromStart)
    (:Update
      (Rendering|Material|SetScalarParameterValue (Variables|Default|GetFadeMaterial) "Fade" _fadevalue :!class /Script/Engine.MaterialInstanceDynamic))
    (:Finished
      (Widget|RemovefromParent (Variables|Default|GetFadeWidget))
      (Default|ClosePauseMenu (Variables|Default|GetCharacter%20Ref)))))

(event EventBeginPlay)

(event Collision|EventActorBeginOverlap
  (params (OtherActor :type Actor%20Object%20Reference)))

(event EventTick
  (params (DeltaSeconds :type Float%20%28single-precision%29)))

(fn ConstructionScript)