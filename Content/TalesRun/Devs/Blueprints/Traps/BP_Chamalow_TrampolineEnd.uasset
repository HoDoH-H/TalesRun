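; Marshmallow trampoline trap that launches the main character when their capsule overlaps its trigger, replacing vertical velocity with the launch force.
; With DoStopMovement, it freezes the character during the full squash animation, then re-enables movement and launches.
; Otherwise it sets velocity to max walk speed along world X and launches immediately with a push-only animation.
; Timelines lerp the cube's scale and position, chaining into a restore timeline.
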(event OnComponentBeginOverlap(TriggerEffect)
  (params (OverlappedComponent :type Primitive%20Component%20Object%20Reference) (OtherActor :type Actor%20Object%20Reference) (OtherComp :type Primitive%20Component%20Object%20Reference) (OtherBodyIndex :type Integer) (bFromSweep :type Boolean) (SweepResult :type Hit%20Result%20Structure%20%28by%20ref%29))
  (bind _cube (Variables|Default|GetCube))
  (bind _cube_2 (Variables|Default|GetCube))
  (bind _base_pos (Variables|Default|GetBase%20Pos))
  (bind _base_pos_2 (Variables|Default|GetBase%20Pos))
  (bind _cube_3 (Variables|Default|GetCube))
  (bind _base_pos_3 (Variables|Default|GetBase%20Pos))
  (bind _base_scale (Variables|Default|GetBase%20Scale))
  (bind (_castsuccess _iscapsulecomponent _characterref) (CallFunction|CasttoMainCharacter OtherActor OtherComp))
  (if _iscapsulecomponent
    (if (Variables|Default|GetDoStopMovement)
      (Variables|/Game/TalesRun/Devs/Blueprints/BP_Character_Devi.BP_Character_Devi_C|SetCanMove? _characterref false)
      (bind (_direction _scale _position) (Timeline|Full%20Anim PlayFromStart)
        (:Update
          (Transformation|SetRelativeScale3D _cube_2 (Math|Vector|Lerp(Vector) _base_scale "1.800000,1.800000,1.000000" _scale) :!label _label)
          (Transformation|SetRelativeLocation _cube_2 (Math|Vector|Lerp(Vector) _base_pos (+ _base_pos "0.000000,0.000000,50.000000") _position) false false))
        (:Finished
          (Utilities|FlowControl|Sequence
            (:then_0
              (goto _label))
            (:then_1
              (Variables|/Game/TalesRun/Devs/Blueprints/BP_Character_Devi.BP_Character_Devi_C|SetCanMove? _characterref true)
              (Character|LaunchCharacter _characterref (Variables|Default|GetLaunchForce) false true)
              (bind (_direction_2 _scale_2 _position_2) (Timeline|Restore%20Initial%20State PlayFromStart)
                (:Update
                  _)
                (:Finished
                  _))
              (Transformation|SetRelativeScale3D _cube (Math|Vector|Lerp(Vector) (Variables|Default|GetBase%20Scale) "1.800000,1.800000,1.000000" _scale_2))
              (Transformation|SetRelativeLocation _cube (Math|Vector|Lerp(Vector) _base_pos_2 (+ _base_pos_2 "0.000000,0.000000,50.000000") _position_2) false false)))))
      (else
        (Variables|/Script/Engine.MovementComponent|SetVelocity (Variables|/Script/Engine.Character|GetCharacterMovement _characterref) (Math|Vector|MakeVector (Variables|/Script/Engine.CharacterMovementComponent|GetMaxWalkSpeed (Variables|/Script/Engine.Character|GetCharacterMovement _characterref)) 0.0 0.0))
        (Character|LaunchCharacter _characterref (Variables|Default|GetLaunchForce) false true)
        (bind (_direction_3 _scale_3 _position_3) (Timeline|Push%20Only%20Anim PlayFromStart)
          (:Update
            (Transformation|SetRelativeScale3D _cube_3 (Math|Vector|Lerp(Vector) _base_scale "1.800000,1.800000,1.000000" _scale_3) :!label _label_2)
            (Transformation|SetRelativeLocation _cube_3 (Math|Vector|Lerp(Vector) _base_pos_3 (+ _base_pos_3 "0.000000,0.000000,50.000000") _position_3) false false))
          (:Finished
            (Utilities|FlowControl|Sequence
              (:then_0
                (goto _label_2))
              (:then_1
                (Timeline|Restore%20Initial%20State PlayFromStart)))))))))

(event EventBeginPlay
  (bind _cube (Variables|Default|GetCube))
  (Variables|Default|SetBase%20Scale (Variables|/Script/Engine.SceneComponent|GetRelativeScale3D _cube))
  (Variables|Default|SetBase%20Pos (Variables|/Script/Engine.SceneComponent|GetRelativeLocation _cube)))

(fn ConstructionScript)