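; BP_Trap_Rolling is a trap actor whose static mesh rolls along a straight path when its Roll event fires.
; Roll caches the mesh's world location, then a timeline linearly moves it a fixed distance along negative world X while ramping pitch toward the Rotation variable.
; When the timeline finishes, the mesh teleports back to its start location with zeroed rotation.
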(event Custom|Roll
  (bind _staticmesh (Variables|Default|GetStaticMesh))
  (Variables|Default|SetBaseLocation (Transformation|GetWorldLocation _staticmesh))
  (bind _newtrack_0 (Timeline|Timeline PlayFromStart)
    (:Update
      (Transformation|SetWorldLocationAndRotation _staticmesh (Math|Interpolation|Ease "Linear" _newtrack_0 (Variables|Default|GetBaseLocation) (- (Variables|Default|GetBaseLocation) "5000.000000,0.000000,0.000000")) (Math|Rotator|MakeRotator 0.0 (Math|Interpolation|Ease "Linear" _newtrack_0 0.0 (Variables|Default|GetRotation)) 0.0) false false))
    (:Finished
      (Transformation|SetWorldLocationAndRotation _staticmesh (Variables|Default|GetBaseLocation) "0, 0, 0" false true))))

(event EventBeginPlay
  (|CallParentFunction) ; This node is disabled and will not be called.\nDrag off pins to build functionality.
)

(event Collision|EventActorBeginOverlap
  (params (OtherActor :type Actor%20Object%20Reference))
  (|CallParentFunction OtherActor) ; This node is disabled and will not be called.\nDrag off pins to build functionality.
)

(event EventTick
  (params (DeltaSeconds :type Float%20%28single-precision%29))
  (|CallParentFunction DeltaSeconds) ; This node is disabled and will not be called.\nDrag off pins to build functionality.
)

(fn ConstructionScript
  (|CallParentFunction))