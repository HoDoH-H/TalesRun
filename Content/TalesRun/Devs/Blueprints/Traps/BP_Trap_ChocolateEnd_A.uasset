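; Chocolate trap that endlessly rises and drops and knocks the main character back with a bounce hit.
; From BeginPlay, UpDownChocolate chains the GoUp and GoDown timelines to drive the mesh's relative Z.
; Short random delays follow each stroke before the event calls itself again, so the rhythm varies.
; Box1 overlaps trigger GetHitWithBounce only when the main character's capsule component enters.
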(event OnComponentBeginOverlap(Box1)
  (params (OverlappedComponent :type Primitive%20Component%20Object%20Reference) (OtherActor :type Actor%20Object%20Reference) (OtherComp :type Primitive%20Component%20Object%20Reference) (OtherBodyIndex :type Integer) (bFromSweep :type Boolean) (SweepResult :type Hit%20Result%20Structure%20%28by%20ref%29))
  (bind (_castsuccess _iscapsulecomponent _characterref) (CallFunction|CasttoMainCharacter OtherActor OtherComp))
  (if _iscapsulecomponent
    (Default|GetHitwithBounce _characterref)))

(event Custom|UpDownChocolate
  (bind _newtrack_0 (Timeline|GoUp PlayFromStart)
    (:Update
      (Transformation|SetRelativeLocation (Variables|Default|GetStaticMesh) (Math|Vector|MakeVector 0.0 0.0 _newtrack_0) false false))
    (:Finished
      (Utilities|FlowControl|Delay (Math|Random|RandomFloatinRange 0.1 0.2))
      (bind _newtrack_0_2 (Timeline|GoDown PlayFromStart)
        (:Update
          (Transformation|SetRelativeLocation (Variables|Default|GetStaticMesh) (Math|Vector|MakeVector 0.0 0.0 _newtrack_0_2) false false))
        (:Finished
          (Utilities|FlowControl|Delay (Math|Random|RandomFloatinRange 0.0 0.5))
          (CallFunction|UpDownChocolate))))))

(event EventBeginPlay
  (|CallParentFunction)
  (CallFunction|UpDownChocolate))

(event Collision|EventActorBeginOverlap
  (params (OtherActor :type Actor%20Object%20Reference))
  (|CallParentFunction OtherActor) ; This node is disabled and will not be called.\nDrag off pins to build functionality.
)

(event EventTick
  (params (DeltaSeconds :type Float%20%28single-precision%29))
  (|CallParentFunction DeltaSeconds) ; This node is disabled and will not be called.\nDrag off pins to build functionality.
)

(fn ConstructionScript
  (|CallParentFunction))