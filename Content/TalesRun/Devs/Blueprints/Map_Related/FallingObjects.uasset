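; Falling object map obstacle that drops and scales a cube when the player character enters its trigger, optionally acting as a trap.
; An outer spawn trigger shows and resets the cube on entry, then hides it and disables its collision on exit.
; The MakeObjectFall timeline lerps location and scale from values cached at BeginPlay, firing once per spawn.
; Non-trap instances destroy their dead zone component at BeginPlay.
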(event OnComponentBeginOverlap(SpawnTrigger)
  (params (OverlappedComponent :type Primitive%20Component%20Object%20Reference) (OtherActor :type Actor%20Object%20Reference) (OtherComp :type Primitive%20Component%20Object%20Reference) (OtherBodyIndex :type Integer) (bFromSweep :type Boolean) (SweepResult :type Hit%20Result%20Structure%20%28by%20ref%29))
  (Utilities|Casting|CastToBP_Character_Devi OtherActor)
  (if (not (Variables|Default|GetIsSpawned))
    (CallFunction|Activate true)
    (Transformation|SetRelativeLocation (Variables|Default|GetCube) (Variables|Default|GetBeginPos) false false)
    (Variables|Default|SetHasFallen false)
    (Variables|Default|SetIsSpawned true)))

(event OnComponentEndOverlap(SpawnTrigger)
  (params (OverlappedComponent :type Primitive%20Component%20Object%20Reference) (OtherActor :type Actor%20Object%20Reference) (OtherComp :type Primitive%20Component%20Object%20Reference) (OtherBodyIndex :type Integer))
  (Utilities|Casting|CastToBP_Character_Devi OtherActor)
  (if (Variables|Default|GetIsSpawned)
    (CallFunction|Activate false)
    (Variables|Default|SetIsSpawned false)))

(event OnComponentBeginOverlap(Trigger)
  (params (OverlappedComponent :type Primitive%20Component%20Object%20Reference) (OtherActor :type Actor%20Object%20Reference) (OtherComp :type Primitive%20Component%20Object%20Reference) (OtherBodyIndex :type Integer) (bFromSweep :type Boolean) (SweepResult :type Hit%20Result%20Structure%20%28by%20ref%29))
  (bind _maxfallscaling (Variables|Default|GetMaxFallScaling))
  (bind _cube (Variables|Default|GetCube))
  (bind _beginscale (Variables|Default|GetBeginScale))
  (bind (_x _y _z) (Math|Vector|BreakVector _beginscale))
  (Utilities|Casting|CastToBP_Character_Devi OtherActor)
  (if (not (Variables|Default|GetHasFallen))
    (bind (_direction _falling _scaling) (Timeline|Make%20Object%20Fall PlayFromStart)
      (:Update
        _)
      (:Finished
        (Variables|Default|SetHasFallen true)))
    (Transformation|SetRelativeLocation _cube (Math|Vector|Lerp(Vector) (Variables|Default|GetBeginPos) (Math|Vector|MakeVector 0.0 0.0 (Variables|Default|GetEndPos)) _falling) false false)
    (Transformation|SetRelativeScale3D _cube (Math|Vector|Lerp(Vector) _beginscale (Math|Vector|MakeVector (+ _x (.x _maxfallscaling)) (+ _y (.y _maxfallscaling)) (+ _z (.z _maxfallscaling))) _scaling))))

(event Custom|Activate
  (params (DoActivate :type Boolean))
  (bind _cube (Variables|Default|GetCube))
  (bind _trigger (Variables|Default|GetTrigger))
  (bind _cube_2 (Variables|Default|GetCube))
  (if DoActivate
    (Collision|SetCollisionEnabled _cube_2 "QueryAndPhysics")
    (Development|SetHiddeninGame _cube false false)
    (Collision|SetCollisionEnabled _trigger "QueryAndPhysics")
    (else
      (Collision|SetCollisionEnabled _cube_2 "NoCollision")
      (Development|SetHiddeninGame _cube true false)
      (Collision|SetCollisionEnabled _trigger "NoCollision"))))

(event EventBeginPlay
  (Variables|Default|SetBeginScale (Variables|/Script/Engine.SceneComponent|GetRelativeScale3D (Variables|Default|GetCube)))
  (Variables|Default|SetBeginPos (Variables|/Script/Engine.SceneComponent|GetRelativeLocation (Variables|Default|GetCube)))
  (if (not (Variables|Default|GetIsTrap))
    (Components|DestroyComponent (Variables|Default|GetBP_DeadZone))))

(fn ConstructionScript)