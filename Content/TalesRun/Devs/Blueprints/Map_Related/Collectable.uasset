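; Collectable pickup actor that acts as either a candy or a power-up, chosen by the IsPowerUp flag.
; On BeginPlay it shows the matching mesh and hides the other.
; Overlap by BP_Character_Devi adds ScoreValue to Score, and also to CandyCollectedNumber for candy, with no power-up effect applied here.
; Pickup only hides both meshes, so the actor remains and can score again on another overlap.
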(event EventBeginPlay
  ;[0.05035 0.05035 0.05035] Change Mesh Based on Type
  (if (Variables|Default|GetIsPowerUp)
    (Rendering|SetVisibility (Variables|Default|GetCandyMesh) false false)
    (Rendering|SetVisibility (Variables|Default|GetPowerUpMesh) true false)
    (else
      (Rendering|SetVisibility (Variables|Default|GetCandyMesh) true false)
      (Rendering|SetVisibility (Variables|Default|GetPowerUpMesh) false false))))

(event Collision|EventActorBeginOverlap
  (params (OtherActor :type Actor%20Object%20Reference))
  (bind _asbp_character_devi (Utilities|Casting|CastToBP_Character_Devi OtherActor))
  (Utilities|FlowControl|Sequence
    (:then_0
      (if (not (Variables|Default|GetIsPowerUp))
        (Variables|/Game/TalesRun/Devs/Blueprints/BP_Character_Devi.BP_Character_Devi_C|SetCandyCollectedNumber _asbp_character_devi (+ (Variables|/Game/TalesRun/Devs/Blueprints/BP_Character_Devi.BP_Character_Devi_C|GetCandyCollectedNumber _asbp_character_devi) (Variables|Default|GetScoreValue)))))
    (:then_1
      (Rendering|SetVisibility (Variables|Default|GetCandyMesh) false false)
      (Rendering|SetVisibility (Variables|Default|GetPowerUpMesh) false false))
    (:then_2
      (Variables|/Game/TalesRun/Devs/Blueprints/BP_Character_Devi.BP_Character_Devi_C|SetScore _asbp_character_devi (+ (Variables|Default|GetScoreValue) (Variables|/Game/TalesRun/Devs/Blueprints/BP_Character_Devi.BP_Character_Devi_C|GetScore _asbp_character_devi))))))

(fn ConstructionScript)