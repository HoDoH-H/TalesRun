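; Blueprint function library for TalesRun with shared helpers for player detection and level transitions.
; CastToMainCharacter casts an actor to BP_Character_Devi and reports whether the given component is its capsule.
; OpenLevelByName stores the CountBeforeStart flag in GI_Custom, then resets health and score when it is set or carries them over from the pawn otherwise.
; The level opens even if the game instance cast fails.
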(fn CasttoMainCharacter
  (params (Actor :type Actor%20Object%20Reference) (Component :type Primitive%20Component%20Object%20Reference))
  (bind _asbp_character_devi (Utilities|Casting|CastToBP_Character_Devi Actor)
    (:then
      (return true (== Component (Variables|/Script/Engine.Character|GetCapsuleComponent _asbp_character_devi)) _asbp_character_devi))
    (:CastFailed
      (return false false 0))))

(fn OpenLevelbyName
  (params (LevelName :type Name) (CountBeforeStart? :type Boolean))
  (bind _asgi_custom (Utilities|Casting|CastToGI_Custom (Game|GetGameInstance))
    (:then
      (LocalVariables|SetGI%20Custom _asgi_custom)
      (bind _output_get (Variables|/Game/TalesRun/Devs/Blueprints/Function_Library/GI_Custom.GI_Custom_C|SetCountBeforeStart? (LocalVariables|GetGI%20Custom) CountBeforeStart?))
      (if _output_get
        (Variables|/Game/TalesRun/Devs/Blueprints/Function_Library/GI_Custom.GI_Custom_C|SetCurrentHealth (LocalVariables|GetGI%20Custom) (Variables|/Game/TalesRun/Devs/Blueprints/Function_Library/GI_Custom.GI_Custom_C|GetDefaultHealth (LocalVariables|GetGI%20Custom)) :!label _label)
        (Variables|/Game/TalesRun/Devs/Blueprints/Function_Library/GI_Custom.GI_Custom_C|SetCurrentScore (LocalVariables|GetGI%20Custom) 0)
        (else
          (bind _asbp_character_devi (Utilities|Casting|CastToBP_Character_Devi (Pawn|GetControlledPawn (Game|GetPlayerController 0)))
            (:then
              (Variables|/Game/TalesRun/Devs/Blueprints/Function_Library/GI_Custom.GI_Custom_C|SetCurrentHealth (LocalVariables|GetGI%20Custom) (Variables|/Game/TalesRun/Devs/Blueprints/BP_Character_Devi.BP_Character_Devi_C|GetCurrentHealth _asbp_character_devi))
              (Variables|/Game/TalesRun/Devs/Blueprints/Function_Library/GI_Custom.GI_Custom_C|SetCurrentScore (LocalVariables|GetGI%20Custom) (Variables|/Game/TalesRun/Devs/Blueprints/BP_Character_Devi.BP_Character_Devi_C|GetScore _asbp_character_devi)))
            (:CastFailed
              (goto _label))))))
    (:CastFailed
      (Development|PrintString 0 "Cast failed to Game Instance" true true "(R=1.000000,G=0.000000,B=0.081652,A=1.000000)" 3.5)))
  (Game|OpenLevel(byName) 0 LevelName))