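; Base platform actor that can fall and interact with whatever it drops onto.
; Fall drives a Timeline that linearly lowers the root by up to 1500 units from its current location.
; While falling, Box overlaps stop the drop on another platform, or bounce-hit the main character via its capsule and destroy this platform.
; Each falling overlap case prints a debug string.
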(event OnComponentBeginOverlap(StaticMesh)
  (params (OverlappedComponent :type Primitive%20Component%20Object%20Reference) (OtherActor :type Actor%20Object%20Reference) (OtherComp :type Primitive%20Component%20Object%20Reference) (OtherBodyIndex :type Integer) (bFromSweep :type Boolean) (SweepResult :type Hit%20Result%20Structure%20%28by%20ref%29)))

(event OnComponentBeginOverlap(Box)
  (params (OverlappedComponent :type Primitive%20Component%20Object%20Reference) (OtherActor :type Actor%20Object%20Reference) (OtherComp :type Primitive%20Component%20Object%20Reference) (OtherBodyIndex :type Integer) (bFromSweep :type Boolean) (SweepResult :type Hit%20Result%20Structure%20%28by%20ref%29))
  (bind _baselocation (Variables|Default|GetbaseLocation))
  (if (Variables|Default|GetisFalling)
    (Utilities|Casting|CastToBP_Platform_Base OtherActor
      (:then
        (Development|PrintString "FALL ON PLATFORM")
        (Variables|Default|SetisFalling false)
        (bind _newtrack_0 (Timeline|Timeline Stop)
          (:Update
            (Transformation|SetWorldLocation (Variables|Default|GetDefaultSceneRoot) (Math|Vector|MakeVector (.x _baselocation) (.y _baselocation) (Math|Interpolation|Ease "Linear" _newtrack_0 (.z _baselocation) (- (.z _baselocation) 1.5e+03))) false false))
          (:Finished
            (Variables|Default|SetisFalling false))))
      (:CastFailed
        (bind (_castsuccess _iscapsulecomponent _characterref) (CallFunction|CasttoMainCharacter OtherActor OtherComp))
        (if _iscapsulecomponent
          (Development|PrintString "FALL ON PLAYER")
          (Default|GetHitwithBounce _characterref)
          (Variables|Default|SetisFalling false)
          (Actor|DestroyActor)
          (else
            (Development|PrintString "FALL ON NOTHING")))))))

(event Custom|Fall
  (Variables|Default|SetbaseLocation (Transformation|GetWorldLocation (Variables|Default|GetDefaultSceneRoot)))
  (Variables|Default|SetisFalling true)
  (bind _newtrack_0 (Timeline|Timeline PlayFromStart)
    (:Update
      (Transformation|SetWorldLocation (Variables|Default|GetDefaultSceneRoot) (Math|Vector|MakeVector (.x (Variables|Default|GetbaseLocation)) (.y (Variables|Default|GetbaseLocation)) (Math|Interpolation|Ease "Linear" _newtrack_0 (.z (Variables|Default|GetbaseLocation)) (- (.z (Variables|Default|GetbaseLocation)) 1.5e+03))) false false))
    (:Finished
      (Variables|Default|SetisFalling false))))

(event EventBeginPlay)

(event Collision|EventActorBeginOverlap
  (params (OtherActor :type Actor%20Object%20Reference)))

(event EventTick
  (params (DeltaSeconds :type Float%20%28single-precision%29)))

(fn ConstructionScript)