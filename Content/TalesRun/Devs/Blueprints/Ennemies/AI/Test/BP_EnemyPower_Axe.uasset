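; BP_EnemyPower_Axe is an enemy axe projectile that flies in an arc across the X/Z plane.
; Fire chains two timelines on the mesh: one rises by ForceHeight, the next descends to the destination.
; Overlapping the main character's capsule triggers a bouncing hit and destroys the axe; otherwise it is destroyed shortly after landing.
; Destroy spawns an effect system at the actor's location before removing it.
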(event OnComponentBeginOverlap(Box)
  (params (OverlappedComponent :type Primitive%20Component%20Object%20Reference) (OtherActor :type Actor%20Object%20Reference) (OtherComp :type Primitive%20Component%20Object%20Reference) (OtherBodyIndex :type Integer) (bFromSweep :type Boolean) (SweepResult :type Hit%20Result%20Structure%20%28by%20ref%29))
  (bind (_castsuccess _iscapsulecomponent _characterref) (CallFunction|CasttoMainCharacter OtherActor OtherComp))
  (if _iscapsulecomponent
    (Default|GetHitwithBounce _characterref)
    (CallFunction|Destroy)))

(event Custom|Destroy
  (Development|PrintString "destroy")
  (Niagara|SpawnSystematLocation "/Game/VFX/Collectibles/Item.Item" (Transformation|GetActorLocation))
  (Utilities|FlowControl|Delay 0.02)
  (Actor|DestroyActor))

(event Custom|Fire
  (params (Destination :type Vector) (BaseLocation :type Vector))
  (Variables|Default|SetXDestination (.x Destination))
  (Variables|Default|SetZDestination (.z Destination))
  (Variables|Default|SetbaseLocX (.x BaseLocation))
  (Variables|Default|SetbasLocZ (.z BaseLocation))
  (bind (_direction _xaxis _zaxis) (Timeline|Timeline_0 PlayFromStart)
    (:Update
      (Transformation|SetWorldLocationAndRotation (Variables|Default|GetStaticMesh) (Math|Vector|MakeVector (Math|Interpolation|Ease "Linear" _xaxis (Variables|Default|GetbaseLocX) (Variables|Default|GetXDestination)) 0.0 (Math|Interpolation|Ease "Linear" _zaxis (Variables|Default|GetbasLocZ) (+ (Variables|Default|GetbasLocZ) (Variables|Default|GetForceHeight)))) (Math|Rotator|MakeRotator 0.0 0.0 0.0) false false))
    (:Finished
      (bind (_direction_2 _xaxis_2 _zaxis_2) (Timeline|Timeline PlayFromStart)
        (:Update
          (Transformation|SetWorldLocationAndRotation (Variables|Default|GetStaticMesh) (Math|Vector|MakeVector (Math|Interpolation|Ease "Linear" _xaxis_2 (Variables|Default|GetbaseLocX) (Variables|Default|GetXDestination)) 0.0 (Math|Interpolation|Ease "Linear" _zaxis_2 (+ (Variables|Default|GetbasLocZ) (Variables|Default|GetForceHeight)) (Variables|Default|GetZDestination))) (Math|Rotator|MakeRotator 0.0 0.0 0.0) false false))
        (:Finished
          (Utilities|FlowControl|Delay 1.5)
          (CallFunction|Destroy))))))

(fn ConstructionScript)