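; Test enemy actor that stays pinned relative to the left screen edge and throws axes at a given destination.
; Each Tick it deprojects that screen edge to world space, subtracts a horizontal offset and raises its height.
; BeginPlay picks that offset once from three viewport aspect-ratio tiers via CalculateCameraOffset.
; Fire spawns a BP_EnemyPower_Axe ahead of the actor and launches it toward the destination; Aim is an empty stub.
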(event Custom|Fire
  (params (Destination :type Vector))
  (bind _returnvalue (Transformation|GetActorLocation))
  (bind _returnvalue_2 (+ (.x _returnvalue) 1e+02))
  (Development|PrintString "FIRE")
  (bind _returnvalue_3 (Game|SpawnActorfromClass "/Game/TalesRun/Devs/Blueprints/Ennemies/AI/Test/BP_EnemyPower_Axe.BP_EnemyPower_Axe_C" (Math|Transform|MakeTransform (Math|Vector|MakeVector _returnvalue_2 0.0 (.z _returnvalue)) "0, 0, 0" "1.500000,1.500000,1.500000") "AdjustIfPossibleButAlwaysSpawn" "MultiplyWithRoot" 0 0))
  (Default|Fire _returnvalue_3 Destination (Math|Vector|MakeVector _returnvalue_2 0.0 (.z _returnvalue))))

(event Custom|Aim)

(event EventBeginPlay
  (bind _output (CallFunction|CalculateCameraOffset))
  (Variables|Default|SetoffsetX _output))

(event Collision|EventActorBeginOverlap
  (params (OtherActor :type Actor%20Object%20Reference)))

(event EventTick
  (params (DeltaSeconds :type Float%20%28single-precision%29))
  (bind _returnvalue (Game|GetPlayerController 0))
  (bind _worldlocation (Class|PlayerController|DeprojectScreenPositiontoWorld _returnvalue -1.0 0.0))
  (Transformation|SetActorLocation (Math|Vector|MakeVector (- (.x _worldlocation) (Variables|Default|GetoffsetX)) 0.0 (+ (.z _worldlocation) 1e+02)) false false))

(fn ConstructionScript)

(fn CalculateCameraOffset
  (bind _returnvalue (Viewport|GetViewportSize))
  (bind _returnvalue_2 (/ (.x _returnvalue) (.y _returnvalue)))
  ;[1 0.7299 0 1 30] ScreenRatio ~ 1920/1080
  (if (> _returnvalue_2 1.75)
    (return 1.1e+03)
    (else
      ;[1 0.7299 0 1 30] ScreenRatio ~ 1520/1080
      (if (> _returnvalue_2 1.4)
        (return 7.8e+02)
        (else
          ;[1 0.7299 0 1 30] ScreenRatio Lesser than 1520/1080
          (return 525.0))))))