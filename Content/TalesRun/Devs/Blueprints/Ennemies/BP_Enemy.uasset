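; BP_Enemy is an enemy that tracks the screen edge, advancing to attack and retreating afterward.
; A looping timer pins it relative to the deprojected top-left screen corner, using an X offset chosen by aspect ratio.
; Prepare eases it forward through a Timeline, enabling Fire to launch a BP_EnemyPower_Axe before a delayed retreat.
; Overlapping a BP_PowerUpTrap halts the advance, disables attacking and sends it back after a delay.
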(event OnComponentBeginOverlap(CapsuleComponent)
  (params (OverlappedComponent :type Primitive%20Component%20Object%20Reference) (OtherActor :type Actor%20Object%20Reference) (OtherComp :type Primitive%20Component%20Object%20Reference) (OtherBodyIndex :type Integer) (bFromSweep :type Boolean) (SweepResult :type Hit%20Result%20Structure%20%28by%20ref%29))
  (Utilities|Casting|CastToBP_PowerUpTrap OtherActor)
  (CallFunction|StopGoFront)
  (Variables|Default|SetcanAttack? false)
  (Utilities|FlowControl|Delay 2.0)
  (CallFunction|GoBack))

(event Custom|StopBacking
  (bind _offset (Timeline|Timeline Stop)
    (:Update
      (Variables|Default|SetoffsetX (Math|Interpolation|Ease "Linear" _offset (Variables|Default|GetcurrentOffsetX) (Variables|Default|GetoffsetBack))))))

(event Custom|Prepare
  (CallFunction|StopBacking)
  (CallFunction|GoFront))

(event Custom|GoFront
  (Variables|Default|SetcurrentOffsetX (Variables|Default|GetoffsetX))
  (bind _offset (Timeline|Timeline_0 PlayFromStart)
    (:Update
      (Variables|Default|SetoffsetX (Math|Interpolation|Ease "Linear" _offset (Variables|Default|GetcurrentOffsetX) (Variables|Default|GetoffsetFront))))
    (:Finished
      (Variables|Default|SetcanAttack? true))))

(event Custom|GoBack
  (Variables|Default|SetcanAttack? false)
  (Variables|Default|SetcurrentOffsetX (Variables|Default|GetoffsetX))
  (bind _offset (Timeline|Timeline PlayFromStart)
    (:Update
      (Variables|Default|SetoffsetX (Math|Interpolation|Ease "Linear" _offset (Variables|Default|GetcurrentOffsetX) (Variables|Default|GetoffsetBack))))))

(event Custom|StopGoFront
  (bind _offset (Timeline|Timeline_0 Stop)
    (:Update
      (Variables|Default|SetoffsetX (Math|Interpolation|Ease "Linear" _offset (Variables|Default|GetcurrentOffsetX) (Variables|Default|GetoffsetFront))))
    (:Finished
      (Variables|Default|SetcanAttack? true))))

(event Custom|Fire
  (params (Destination :type Vector))
  (bind _returnvalue (Transformation|GetActorLocation))
  (bind _returnvalue_2 (+ (.x _returnvalue) 1e+02))
  (if (Variables|Default|GetcanAttack?)
    (bind _returnvalue_3 (Game|SpawnActorfromClass "/Game/TalesRun/Devs/Blueprints/Ennemies/BP_EnemyPower_Axe.BP_EnemyPower_Axe_C" (Math|Transform|MakeTransform (Math|Vector|MakeVector _returnvalue_2 0.0 (.z _returnvalue)) "0, 0, 0" "1.500000,1.500000,1.500000") "AdjustIfPossibleButAlwaysSpawn" "MultiplyWithRoot" 0 0))
    (Default|Fire _returnvalue_3 Destination (Math|Vector|MakeVector _returnvalue_2 0.0 (.z _returnvalue)) (Variables|Default|GetforceHeight))
    (Utilities|FlowControl|Delay (Variables|Default|GetdisappearTimer))
    (CallFunction|GoBack)))

(event Custom|AutoRun
  (bind _returnvalue (Game|GetPlayerController 0))
  (bind _worldlocation (Class|PlayerController|DeprojectScreenPositiontoWorld _returnvalue -1.0 0.0))
  (Transformation|SetActorLocation (Math|Vector|MakeVector (- (.x _worldlocation) (Variables|Default|GetoffsetX)) 0.0 (+ (.z _worldlocation) 2e+02)) false false))

(event EventBeginPlay
  (bind (_offsetfront _offsetback) (CallFunction|CalculateCameraOffset))
  (Variables|Default|SetoffsetFront _offsetfront)
  (bind _output_get (Variables|Default|SetoffsetBack _offsetback))
  (bind _output_get_2 (Variables|Default|SetoffsetX _output_get))
  (Variables|Default|SetcurrentOffsetX _output_get_2)
  (Utilities|FlowControl|Delay 0.2)
  (Utilities|Time|SetTimerbyEvent (delegate Custom|AutoRun) 0.01 true))

(event Collision|EventActorBeginOverlap
  (params (OtherActor :type Actor%20Object%20Reference)))

(fn ConstructionScript)

(fn CalculateCameraOffset
  (bind _returnvalue (Viewport|GetViewportSize))
  (bind _returnvalue_2 (/ (.x _returnvalue) (.y _returnvalue)))
  ;[1 0.7299 0 1 30] ScreenRatio ~ 1920/1080
  (if (> _returnvalue_2 1.75)
    (return 1e+03 1.5e+03)
    (else
      ;[1 0.7299 0 1 30] ScreenRatio ~ 1520/1080
      (if (> _returnvalue_2 1.4)
        (return 7.8e+02 1.2e+03)
        (else
          ;[1 0.7299 0 1 30] ScreenRatio Lesser than 1520/1080
          (return 525.0 9.5e+02))))))