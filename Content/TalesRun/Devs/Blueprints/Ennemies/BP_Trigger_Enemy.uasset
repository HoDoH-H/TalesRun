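; BP_Trigger_Enemy is a placed trigger that cues a Hansel or Gretel enemy encounter on the main character.
; Overlapping TriggerPrepare calls the character's arrive event, and overlapping TriggerFire calls its attack event with FinalLocation's world position.
; Only the character's capsule activates either volume.
; The Hansel and Gretel flags pick which events fire, with Hansel taking priority and a debug message printed if neither is set.
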(event OnComponentBeginOverlap(TriggerFire)
  (params (OverlappedComponent :type Primitive%20Component%20Object%20Reference) (OtherActor :type Actor%20Object%20Reference) (OtherComp :type Primitive%20Component%20Object%20Reference) (OtherBodyIndex :type Integer) (bFromSweep :type Boolean) (SweepResult :type Hit%20Result%20Structure%20%28by%20ref%29))
  (bind _finallocation (Variables|Default|GetFinalLocation))
  (bind _returnvalue (Transformation|GetWorldLocation _finallocation))
  (bind (_castsuccess _iscapsulecomponent _characterref) (CallFunction|CasttoMainCharacter OtherActor OtherComp))
  (if _iscapsulecomponent
    (if (Variables|Default|GetHansel)
      (Default|HanselAttackEvent _characterref _returnvalue)
      (elif (Variables|Default|GetGretel)
        (Default|GretelAttackEvent _characterref _returnvalue)
        (else
          (Development|PrintString "Both Hansel & Gretel are not assign on trigger" true true "(R=0.822917,G=0.000000,B=0.005653,A=1.000000)" 5.0))))))

(event OnComponentBeginOverlap(TriggerPrepare)
  (params (OverlappedComponent :type Primitive%20Component%20Object%20Reference) (OtherActor :type Actor%20Object%20Reference) (OtherComp :type Primitive%20Component%20Object%20Reference) (OtherBodyIndex :type Integer) (bFromSweep :type Boolean) (SweepResult :type Hit%20Result%20Structure%20%28by%20ref%29))
  (bind (_castsuccess _iscapsulecomponent _characterref) (CallFunction|CasttoMainCharacter OtherActor OtherComp))
  (if _iscapsulecomponent
    (if (Variables|Default|GetHansel)
      (Default|HanselArriveEvent _characterref)
      (elif (Variables|Default|GetGretel)
        (Default|GretelArriveEvent _characterref)
        (else
          (Development|PrintString "Both Hansel & Gretel are not assign on trigger" true true "(R=0.822917,G=0.000000,B=0.005653,A=1.000000)" 5.0))))))

(event EventBeginPlay)

(event Collision|EventActorBeginOverlap
  (params (OtherActor :type Actor%20Object%20Reference)))

(event EventTick
  (params (DeltaSeconds :type Float%20%28single-precision%29)))

(fn ConstructionScript)