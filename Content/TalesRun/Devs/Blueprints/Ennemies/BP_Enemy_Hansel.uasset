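; BP_Enemy_Hansel is the Hansel enemy, which makes a single bomb attack at a given destination.
; When CanAttack is set, Fire spawns an enlarged BP_EnemyPower_Bomb offset along X from its location and launches it with ForceHeight.
; It then clears CanAttack, waits DisappearTimer and calls GoBack.
; BeginPlay, overlap and Tick are disabled stubs, so Fire is its only active logic.
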(event EventBeginPlay
  (|CallParentFunction) ; This node is disabled and will not be called.\nDrag off pins to build functionality.
)

(event Collision|EventActorBeginOverlap
  (params (OtherActor :type Actor%20Object%20Reference))
  (|CallParentFunction OtherActor) ; This node is disabled and will not be called.\nDrag off pins to build functionality.
)

(event EventTick
  (params (DeltaSeconds :type Float%20%28single-precision%29))
  (|CallParentFunction DeltaSeconds) ; This node is disabled and will not be called.\nDrag off pins to build functionality.
)

(event EventFire
  (params (Destination :type Vector :default "0, 0, 0"))
  (bind _returnvalue (Transformation|GetActorLocation))
  (bind _returnvalue_2 (+ (.x _returnvalue) 1e+02))
  (if (Variables|Default|GetcanAttack?)
    (bind _returnvalue_3 (Game|SpawnActorfromClass "/Game/TalesRun/Devs/Blueprints/Ennemies/BP_EnemyPower_Bomb.BP_EnemyPower_Bomb_C" (Math|Transform|MakeTransform (Math|Vector|MakeVector _returnvalue_2 0.0 (.z _returnvalue)) "0, 0, 0" "1.500000,1.500000,1.500000") "AdjustIfPossibleButAlwaysSpawn" "MultiplyWithRoot" 0 0))
    (Default|Fire _returnvalue_3 Destination (Math|Vector|MakeVector _returnvalue_2 0.0 (.z _returnvalue)) (Variables|Default|GetforceHeight))
    (Variables|Default|SetcanAttack? false)
    (Utilities|FlowControl|Delay (Variables|Default|GetdisappearTimer))
    (CallFunction|GoBack)))

(fn ConstructionScript
  (|CallParentFunction))