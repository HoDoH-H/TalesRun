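; Lollipop trap actor that tips over when the player character Devi enters its trigger.
; On begin play it offsets the trigger box along X by a configurable distance and resets the mesh to its starting rotation.
; When an overlapping actor casts to Devi, a timeline plays from the start and lerps the mesh's roll to a configurable target rotation.
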(event EventBeginPlay
  (Transformation|SetRelativeLocation (Variables|Default|GetBox) (Math|Vector|MakeVector (Variables|Default|GetTrigger%20Distance) 0.0 0.0) false false)
  (Transformation|SetRelativeRotation (Variables|Default|GetCube) "0.000000,-89.999990,-90.000000" false false))

(event Collision|EventActorBeginOverlap
  (params (OtherActor :type Actor%20Object%20Reference))
  (Utilities|Casting|CastToBP_Character_Devi OtherActor)
  (bind _newtrack_0 (Timeline|Timeline PlayFromStart)
    (:Update
      (Transformation|SetRelativeRotation (Variables|Default|GetCube) (Math|Rotator|Lerp(Rotator) (Math|Rotator|MakeRotator -9e+01 0.0 -89.99999) (Math|Rotator|MakeRotator (Variables|Default|GetLollyPop%20Rotation) 0.0 -89.99999) _newtrack_0) false false))))

(fn ConstructionScript)