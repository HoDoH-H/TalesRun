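; BP_ForestBackground1 is a modular, layered forest backdrop built procedurally in the construction script, with no active runtime logic.
; It places copies of one forest mesh at increasing depth along negative Y, each layer using its own material.
; The front layer is a single piece at the top row, two middle layers repeat vertically per Height, and the rear is one Z-stretched piece.
; Scale sizes the pieces and their vertical spacing, while three Depth variables separate the layers.
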(event EventBeginPlay)

(event Collision|EventActorBeginOverlap
  (params (OtherActor :type Actor%20Object%20Reference)))

(event EventTick
  (params (DeltaSeconds :type Float%20%28single-precision%29)))

(fn ConstructionScript
  (bind _scale (Variables|Default|GetScale))
  (bind _scale_2 (Variables|Default|GetScale))
  (bind _scale_3 (Variables|Default|GetScale))
  (bind _scale_4 (Variables|Default|GetScale))
  (Utilities|FlowControl|Sequence
    (:then_0
      ;[1 1 1] Background
      (bind _returnvalue (AddComponent|AddStaticMeshComponent false (Math|Transform|MakeTransform (Math|Vector|MakeVector 0.0 0.0 (* _scale (- (Variables|Default|GetHeight) 1) 3e+01)) "0, 0, 0" (Math|Conversions|ToVector(Float) _scale))))
      (Components|StaticMesh|SetStaticMesh _returnvalue "/Game/TalesRun/3DStuff/Environnement/Assets/BKG/Props/Forest/MOD_SM_Forest.MOD_SM_Forest")
      (Rendering|Material|SetMaterial _returnvalue 0 "/Game/TalesRun/3DStuff/Environnement/Material/BKG/Forest/MI_MOD_ForestBackground_A.MI_MOD_ForestBackground_A"))
    (:then_1
      ;[1 1 1] Boucle Répétition objets
      (for _index (range 0 (- (Variables|Default|GetHeight) 1))
        (bind _returnvalue_2 (AddComponent|AddStaticMeshComponent false (Math|Transform|MakeTransform (Math|Vector|MakeVector 0.0 (- 0.0 (Variables|Default|GetDepthForeground)) (* _index _scale_2 3e+01)) "0, 0, 0" (Math|Conversions|ToVector(Float) _scale_2))))
        (Components|StaticMesh|SetStaticMesh _returnvalue_2 "/Game/TalesRun/3DStuff/Environnement/Assets/BKG/Props/Forest/MOD_SM_Forest.MOD_SM_Forest")
        (Rendering|Material|SetMaterial _returnvalue_2 0 "/Game/TalesRun/3DStuff/Environnement/Material/BKG/Forest/MI_MOD_ForestBackground_B.MI_MOD_ForestBackground_B")
        ;[1 1 1] Boucle Répétition objets
        (bind _returnvalue_3 (AddComponent|AddStaticMeshComponent false (Math|Transform|MakeTransform (Math|Vector|MakeVector 0.0 (Utilities|Operators|Subtract 0.0 (Variables|Default|GetDepthForeground) (Variables|Default|GetDepthMiddleground)) (* _index _scale_3 3e+01)) "0, 0, 0" (Math|Conversions|ToVector(Float) _scale_3))))
        (Components|StaticMesh|SetStaticMesh _returnvalue_3 "/Game/TalesRun/3DStuff/Environnement/Assets/BKG/Props/Forest/MOD_SM_Forest.MOD_SM_Forest")
        (Rendering|Material|SetMaterial _returnvalue_3 0 "/Game/TalesRun/3DStuff/Environnement/Material/BKG/Forest/MI_MOD_ForestBackground_C.MI_MOD_ForestBackground_C")))
    (:then_3
      ;[1 1 1] Background
      (bind _returnvalue_4 (AddComponent|AddStaticMeshComponent false (Math|Transform|MakeTransform (Math|Vector|MakeVector 0.0 (Utilities|Operators|Subtract 0.0 (Variables|Default|GetDepthForeground) (Variables|Default|GetDepthMiddleground) (Variables|Default|GetDepthBackground)) (- 0.0 (Utilities|Operators|Divide _scale_4 2.0 0.03))) "0, 0, 0" (Math|Vector|MakeVector _scale_4 _scale_4 (* (+ (Variables|Default|GetHeight) 1) _scale_4)))))
      (Components|StaticMesh|SetStaticMesh _returnvalue_4 "/Game/TalesRun/3DStuff/Environnement/Assets/BKG/Props/Forest/MOD_SM_Forest.MOD_SM_Forest")
      (Rendering|Material|SetMaterial _returnvalue_4 0 "/Game/TalesRun/3DStuff/Environnement/Material/BKG/Forest/MI_MOD_ForestBackground.MI_MOD_ForestBackground"))))