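; SaveManager saves the player's collected candy count and chrono time to a save slot.
; SaveGame creates a BP_SaveSystem object if none is valid, copies both values from BP_ThirdPersonCharacter and its BPChrono, then writes the slot.
; LoadGame only prints the stored values without applying them to the character or the cached save object, and calls SaveGame when no save exists.
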(fn SaveGame
  (Utilities|FlowControl|Sequence
    (:then_0
      (Utilities|IsValid (Variables|Default|GetSaveSystem)
        (:Is%20Not%20Valid
          (bind _returnvalue (SaveGame|CreateSaveGameObject "/Game/TalesRun/Devs/Blueprints/BP_SaveSystem.BP_SaveSystem_C"))
          (Variables|Default|SetSaveSystem _returnvalue))))
    (:then_1
      (bind _asbp_third_person_character (Utilities|Casting|CastToBP_ThirdPersonCharacter (Game|GetPlayerCharacter 0)))
      (Variables|/Game/TalesRun/Devs/Blueprints/BP_SaveSystem.BP_SaveSystem_C|SetCollectables%20-%201 (Variables|Default|GetSaveSystem) (Variables|/Game/ThirdPerson/Blueprints/BP_ThirdPersonCharacter.BP_ThirdPersonCharacter_C|GetCandyCollectedNumber _asbp_third_person_character))
      (Variables|/Game/TalesRun/Devs/Blueprints/BP_SaveSystem.BP_SaveSystem_C|SetTimer%20-%201%20-%20TimeLeft (Variables|Default|GetSaveSystem) (Variables|/Game/TalesRun/Devs/Blueprints/BP_Chrono.BP_Chrono_C|GetCurrentTime (Variables|/Game/ThirdPerson/Blueprints/BP_ThirdPersonCharacter.BP_ThirdPersonCharacter_C|GetBP_Chrono _asbp_third_person_character))))
    (:then_2
      (SaveGame|SaveGametoSlot (Variables|Default|GetSaveSystem) (Variables|Default|GetSave%20Name)))))

(fn LoadGame
  (bind _save_name (Variables|Default|GetSave%20Name))
  (bind _returnvalue (SaveGame|DoesSaveGameExist _save_name))
  (if _returnvalue
    (bind _returnvalue_2 (SaveGame|LoadGamefromSlot _save_name))
    (bind _asbp_save_system (Utilities|Casting|CastToBP_SaveSystem _returnvalue_2))
    (Development|PrintString (Utilities|String|ToString(Integer) (Variables|/Game/TalesRun/Devs/Blueprints/BP_SaveSystem.BP_SaveSystem_C|GetCollectables%20-%201 _asbp_save_system)))
    (Development|PrintString (Utilities|String|ToString(Float) (Variables|/Game/TalesRun/Devs/Blueprints/BP_SaveSystem.BP_SaveSystem_C|GetTimer%20-%201%20-%20TimeLeft _asbp_save_system)))
    (else
      (CallFunction|SaveGame))))