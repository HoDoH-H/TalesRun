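; SaveManager saves and loads a BP_SaveSystem save object in the slot named by SaveName.
; SaveGame creates the object if missing, casts the player character, then writes the slot; the nodes copying collected candy and chrono time into it are not connected.
; LoadGame prints the stored collectable and timer values without applying them, or calls SaveGame when no save exists.
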(fn SaveGame
  (Utilities|FlowControl|Sequence
    (:then_0
      (Utilities|IsValid (Variables|Default|GetSaveSystem)
        (:Is%20Not%20Valid
          (bind _returnvalue (SaveGame|CreateSaveGameObject "/Game/TalesRun/Blueprints/BP_SaveSystem.BP_SaveSystem_C"))
          (Variables|Default|SetSaveSystem _returnvalue))))
    (:then_1
      (Utilities|Casting|CastToBP_ThirdPersonCharacter (Game|GetPlayerCharacter 0)))
    (:then_2
      (SaveGame|SaveGametoSlot (Variables|Default|GetSaveSystem) (Variables|Default|GetSave%20Name)))))

(fn LoadGame
  (bind _save_name (Variables|Default|GetSave%20Name))
  (bind _returnvalue (SaveGame|DoesSaveGameExist _save_name))
  (if _returnvalue
    (bind _returnvalue_2 (SaveGame|LoadGamefromSlot _save_name))
    (bind _asbp_save_system (Utilities|Casting|CastToBP_SaveSystem _returnvalue_2))
    (Development|PrintString (Utilities|String|ToString(Integer) (Variables|/Game/TalesRun/Blueprints/BP_SaveSystem.BP_SaveSystem_C|GetCollectables%20-%201 _asbp_save_system)))
    (Development|PrintString (Utilities|String|ToString(Float) (Variables|/Game/TalesRun/Blueprints/BP_SaveSystem.BP_SaveSystem_C|GetTimer%20-%201%20-%20TimeLeft _asbp_save_system)))
    (else
      (CallFunction|SaveGame))))