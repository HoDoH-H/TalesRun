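; Oreo is a one-shot triggered actor that moves a cylinder when the BP_Character_Devi player character overlaps it.
; BeginPlay offsets the Box trigger along X by TriggerDistance and resets the Cylinder to the relative origin.
; The overlap destroys the Box and plays a timeline that lerps the Cylinder along X toward OreoAppears, then destroys the Cylinder when finished.
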(event EventBeginPlay
  (Transformation|SetRelativeLocation (Variables|Default|GetBox) (Math|Vector|MakeVector (Variables|Default|GetTrigger%20Distance) 0.0 0.0) false false)
  (Transformation|SetRelativeLocation (Variables|Default|GetCylinder) "0.000000,0.000000,0.000000" false false))

(event Collision|EventActorBeginOverlap
  (params (OtherActor :type Actor%20Object%20Reference))
  (Utilities|Casting|CastToBP_Character_Devi OtherActor)
  (Components|DestroyComponent (Variables|Default|GetBox))
  (bind _newtrack_0 (Timeline|Timeline PlayFromStart)
    (:Update
      (Transformation|SetRelativeLocation (Variables|Default|GetCylinder) (Math|Vector|Lerp(Vector) (Math|Vector|MakeVector 1e+02 0.0 0.0) (Math|Vector|MakeVector (Variables|Default|GetOreo%20Appears) 0.0 0.0) _newtrack_0) false false))
    (:Finished
      (Components|DestroyComponent (Variables|Default|GetCylinder)))))

(fn ConstructionScript)