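; Collectable pickup actor that appears as either a candy or a power-up, chosen by the IsPowerUp flag at BeginPlay.
; Any actor overlap increments CandyCollectedNumber on player 0's BP_ThirdPersonCharacter, regardless of type or overlapping actor, then hides both meshes.
; The actor is neither destroyed nor has its collision disabled, so later overlaps increment the count again.
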(event EventBeginPlay
  ;[0.05035 0.05035 0.05035] Change Mesh Based on Type
  (if (Variables|Default|GetIsPowerUp)
    (Rendering|SetVisibility (Variables|Default|GetCandyMesh) false false)
    (Rendering|SetVisibility (Variables|Default|GetPowerUpMesh) true false)
    (else
      (Rendering|SetVisibility (Variables|Default|GetCandyMesh) true false)
      (Rendering|SetVisibility (Variables|Default|GetPowerUpMesh) false false))))

(event Collision|EventActorBeginOverlap
  (params (OtherActor :type Actor%20Object%20Reference))
  (bind _asbp_third_person_character (Utilities|Casting|CastToBP_ThirdPersonCharacter (Game|GetPlayerCharacter 0)))
  (Variables|/Game/ThirdPerson/Blueprints/BP_ThirdPersonCharacter.BP_ThirdPersonCharacter_C|SetCandyCollectedNumber _asbp_third_person_character (+ (Variables|/Game/ThirdPerson/Blueprints/BP_ThirdPersonCharacter.BP_ThirdPersonCharacter_C|GetCandyCollectedNumber _asbp_third_person_character) 1))
  (Rendering|SetVisibility (Variables|Default|GetCandyMesh) false false)
  (Rendering|SetVisibility (Variables|Default|GetPowerUpMesh) false false))

(fn ConstructionScript)