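; FallingObjects is an actor whose cube falls when the Devi player character overlaps it, optionally acting as a deadly trap.
; BeginPlay caches the cube's starting relative location and scale, and destroys the BPDeadZone component unless IsTrap is set.
; The overlap restarts the MakeObjectFall timeline, whose separate curves lerp the cube toward the EndPos height and toward its starting scale plus MaxFallScaling.
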(event Collision|EventActorBeginOverlap
  (params (OtherActor :type Actor%20Object%20Reference))
  (bind _maxfallscaling (Variables|Default|GetMaxFallScaling))
  (bind _cube (Variables|Default|GetCube))
  (bind _beginscale (Variables|Default|GetBeginScale))
  (bind (_x _y _z) (Math|Vector|BreakVector _beginscale))
  (Utilities|Casting|CastToBP_Character_Devi OtherActor)
  (bind (_direction _falling _scaling) (Timeline|Make%20Object%20Fall PlayFromStart)
    (:Update
      _)
    (:Finished
      _))
  (Transformation|SetRelativeLocation _cube (Math|Vector|Lerp(Vector) (Variables|Default|GetBeginPos) (Math|Vector|MakeVector 0.0 0.0 (Variables|Default|GetEndPos)) _falling) false false)
  (Transformation|SetRelativeScale3D _cube (Math|Vector|Lerp(Vector) _beginscale (Math|Vector|MakeVector (+ _x (.x _maxfallscaling)) (+ _y (.y _maxfallscaling)) (+ _z (.z _maxfallscaling))) _scaling)))

(event EventBeginPlay
  (Variables|Default|SetBeginScale (Variables|/Script/Engine.SceneComponent|GetRelativeScale3D (Variables|Default|GetCube)))
  (Variables|Default|SetBeginPos (Variables|/Script/Engine.SceneComponent|GetRelativeLocation (Variables|Default|GetCube)))
  (if (not (Variables|Default|GetIsTrap))
    (Components|DestroyComponent (Variables|Default|GetBP_DeadZone))))

(fn ConstructionScript)