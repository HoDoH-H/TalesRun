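; Chocolate bar gameplay element that moves into place when the player character, BP_Character_Devi, overlaps the actor.
; BeginPlay offsets the trigger Box by TriggerDistance and starts the Cube at a lowered or raised height depending on IsAscendant.
; On overlap, one of two timelines lerps the Cube's relative Z to ChocolateAppears, so it either rises or descends.
; The timeline restarts on every qualifying overlap, with no one-shot guard.
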(event EventBeginPlay
  (bind _cube (Variables|Default|GetCube))
  (Variables|Default|SetBegin (Variables|/Script/Engine.SceneComponent|GetRelativeScale3D (Variables|Default|GetCube)))
  (Transformation|SetRelativeLocation (Variables|Default|GetBox) (Math|Vector|MakeVector (Variables|Default|GetTrigger%20Distance) 0.0 0.0) false false)
  (if (Variables|Default|GetIsAscendant)
    (Transformation|SetRelativeLocation _cube "0.000000,0.000000,-210.000000" false false)
    (else
      (Transformation|SetRelativeLocation _cube "0.000000,0.000000,100.000000" false false))))

(event Collision|EventActorBeginOverlap
  (params (OtherActor :type Actor%20Object%20Reference))
  (bind _chocolate_appears (Variables|Default|GetChocolate%20Appears))
  (Utilities|Casting|CastToBP_Character_Devi OtherActor)
  (if (Variables|Default|GetIsAscendant)
    (bind _appears (Timeline|Z PlayFromStart)
      (:Update
        (Transformation|SetRelativeLocation (Variables|Default|GetCube) (Math|Vector|Lerp(Vector) (Math|Vector|MakeVector 0.0 0.0 -2.1e+02) (Math|Vector|MakeVector 0.0 0.0 _chocolate_appears) _appears) false false)))
    (else
      (bind _appears_2 (Timeline|Timeline PlayFromStart)
        (:Update
          _)
        (:Finished
          _))
      (Transformation|SetRelativeLocation (Variables|Default|GetCube) (Math|Vector|Lerp(Vector) (Math|Vector|MakeVector 0.0 0.0 1e+02) (Math|Vector|MakeVector 0.0 0.0 _chocolate_appears) _appears_2) false false))))

(fn ConstructionScript)