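; BP_Bonbon is a collectible bonbon pickup that bobs vertically and adds points to the player's score.
; On BeginPlay it reads its selected row from CDT_BonBons to set mesh and point value, then loops a timeline-driven float animation.
; Any sphere overlap plays a sound and Niagara effect, destroys the actor and credits BP_Character_Devi on player pawn 0, without checking the overlapping actor.
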(event OnComponentBeginOverlap(Sphere)
  (params (OverlappedComponent :type Primitive%20Component%20Object%20Reference) (OtherActor :type Actor%20Object%20Reference) (OtherComp :type Primitive%20Component%20Object%20Reference) (OtherBodyIndex :type Integer) (bFromSweep :type Boolean) (SweepResult :type Hit%20Result%20Structure%20%28by%20ref%29))
  (Audio|PlaySound2D (Variables|Default|GetPickUpSound) 1.0 1.0 0.0 0 0)
  (Niagara|SpawnSystematLocation "/Game/VFX/PickUp/NS_PickUpEffect.NS_PickUpEffect" (Transformation|GetWorldLocation (Variables|Default|GetBonbon)))
  (Actor|DestroyActor)
  (bind _asbp_character_devi (Utilities|Casting|CastToBP_Character_Devi (Game|Player|GetPlayerPawn 0)))
  (Variables|/Game/TalesRun/Blueprints/BP_Character_Devi.BP_Character_Devi_C|SetScore _asbp_character_devi (+ (Variables|Default|GetPoints) (Variables|/Game/TalesRun/Blueprints/BP_Character_Devi.BP_Character_Devi_C|GetScore _asbp_character_devi))))

(event Custom|Animation
  (bind _z_axismovement (Timeline|FloatingAnim Play)
    (:Update
      (Transformation|SetRelativeLocation (Variables|Default|GetBonbon) _z_axismovement false false))
    (:Finished
      (bind _z_axismovement_2 (Timeline|Timeline ReverseFromEnd)
        (:Update
          (Transformation|SetRelativeLocation (Variables|Default|GetBonbon) _z_axismovement_2 false false))
        (:Finished
          (Timeline|FloatingAnim PlayFromStart))))))

(event EventBeginPlay
  (CallFunction|FindDTHandleRow)
  (CallFunction|SetVisual)
  (CallFunction|Animation))

(event EventTick
  (params (DeltaSeconds :type Float%20%28single-precision%29)))

(fn ConstructionScript)

(fn SetVisual
  (bind _itemmesh (Variables|Default|GetItemMesh))
  (bind _iteminfo (Variables|Default|GetItemInfo))
  (bind (_mesh _valuepoints) (Utilities|Struct|BreakS_BonbonsPowerUp _iteminfo))
  (bind _array_element (Utilities|Array|ForEachLoopwithBreak _itemmesh)
    (:LoopBody
      (Components|DestroyComponent _array_element))
    (:Completed
      (Utilities|Array|Clear _itemmesh)
      (Utilities|FlowControl|Sequence
        (:then_0
          (Components|StaticMesh|SetStaticMesh (Variables|Default|GetBonbon) _mesh))
        (:then_1
          (Variables|Default|SetPoints _valuepoints))))))

(fn FindDTHandleRow
  (bind _returnvalue (Utilities|GetDataTableRow "/Game/Devs/DataTables/CDT_BonBons.CDT_BonBons" (.RowName (Utilities|Struct|BreakDataTableRowHandle (Utilities|Struct|BreakS_BonBons (Variables|Default|GetSelectedItem)))))
    (:then
      (Variables|Default|SetItemInfo _returnvalue))))