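; Chocolate bar trap that hits the main character with a bounce when their capsule enters its Box trigger.
; On BeginPlay it applies one of three materials at random to the static mesh for visual variety.
; Timeline logic for making the bar rise or descend into view, chosen by IsAscendant, is present but disconnected and never runs.
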(event OnComponentBeginOverlap(Box)
  (params (OverlappedComponent :type Primitive%20Component%20Object%20Reference) (OtherActor :type Actor%20Object%20Reference) (OtherComp :type Primitive%20Component%20Object%20Reference) (OtherBodyIndex :type Integer) (bFromSweep :type Boolean) (SweepResult :type Hit%20Result%20Structure%20%28by%20ref%29))
  (bind (_castsuccess _iscapsulecomponent _characterref) (CallFunction|CasttoMainCharacter OtherActor OtherComp))
  (if _iscapsulecomponent
    (Default|GetHitwithBounce _characterref)))

(event EventBeginPlay
  (CallFunction|RandomTexture))

(fn ConstructionScript)

(fn RandomTexture
  (bind _textures (Variables|Default|GetTextures))
  (Rendering|Material|SetMaterial (Variables|Default|GetStaticMesh) 0 (Utilities|Select :Index (Math|Random|RandomIntegerinRange 0 2) :Option%200 (Utilities|Array|Get(acopy) _textures) :Option%201 (Utilities|Array|Get(acopy) _textures 1) :Option%202 (Utilities|Array|Get(acopy) _textures 2))))